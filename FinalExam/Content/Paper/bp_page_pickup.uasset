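; Collectible page pickup actor that counts toward the player's total and triggers victory on the eighth page.
; When the first-person character overlaps the Paper1 component, it disables that component's collision and reads NumPages from the first BP_FirstPersonCharacter found in the level.
; It either increments that count and destroys itself, or, on the final page, adds the Victory widget to the viewport and pauses the game.
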(event `self.paper1.OnComponentBeginOverlap`
  (params (OverlappedComponent :type "PrimitiveComponent Object Reference") (OtherActor :type "Actor Object Reference") (OtherComp :type "PrimitiveComponent Object Reference") (OtherBodyIndex :type Integer) (bFromSweep :type Boolean) (SweepResult :type "HitResult Structure (by ref)"))
  (cast `/Game/ThirdPerson/Blueprints/BP_FirstPersonCharacter` OtherActor)
  (`PrimitiveComponent.SetCollisionEnabled` (`self.paper1`) "NoCollision")
  (bind _outactors (`GameplayStatics.GetAllActorsOfClass` "/Game/ThirdPerson/Blueprints/BP_FirstPersonCharacter.BP_FirstPersonCharacter_C"))
  (bind _output (`|GetArrayItem` _outactors))
  (bind _returnvalue (+ (`/Game/ThirdPerson/Blueprints/BP_FirstPersonCharacter.num pages` _output) 1))
  (if (== _returnvalue 8)
    (bind _returnvalue_2 (`|CreateWidget` "/Game/victory.victory_C"))
    (`UserWidget.AddToViewport` _returnvalue_2 0)
    (`GameplayStatics.SetGamePaused` true)
    (else
      (set `/Game/ThirdPerson/Blueprints/BP_FirstPersonCharacter.num pages` _returnvalue _output)
      (`self.K2_DestroyActor`))))

(fn `UserConstructionScript`)