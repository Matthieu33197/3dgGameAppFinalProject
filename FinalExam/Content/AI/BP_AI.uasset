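; AI pawn that detects the player and delivers a melee attack.
; Pawn sensing sets the SeeingPlayer blackboard key for Player-tagged pawns, and a looping one-second timer clears it.
; AttackPlayer, guarded by an Attacking flag, plays a montage and sphere-traces forward from AttackTracePoint for pawns, applying fixed damage to the hit actor.
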(event `self.ReceiveBeginPlay`
  (`KismetSystemLibrary.K2_SetTimerDelegate` (delegate `Stop seeing player`) 1.0 true))

(event `Stop seeing player`
  (`BlackboardComponent.SetValueAsBool` (`AIBlueprintHelperLibrary.GetBlackboard` (`AIBlueprintHelperLibrary.GetAIController` self)) "SeeingPlayer" false))

(event `self.PawnSensing.OnSeePawn`
  (params (Pawn :type "Pawn Object Reference"))
  (if (`self.ActorHasTag` Pawn "Player")
    (`BlackboardComponent.SetValueAsBool` (`AIBlueprintHelperLibrary.GetBlackboard` (`AIBlueprintHelperLibrary.GetAIController` self)) "SeeingPlayer" true)))

(event `AttackPlayer`
  (bind _attack_trace_point (`self.attack trace point`))
  (bind _returnvalue (`SceneComponent.K2_GetComponentLocation` _attack_trace_point))
  (if (not (`self.attacking?`))
    (set `self.attacking?` true)
    (`|PlayMontage` null
      (:`then`
        (set `self.attacking?` false)
        (bind (_outhit _returnvalue_2) (`KismetSystemLibrary.SphereTraceSingleForObjects` _returnvalue (+ _returnvalue (* (`KismetMathLibrary.GetForwardVector` (`SceneComponent.K2_GetComponentRotation` _attack_trace_point)) 200.0)) 50.0 (`|MakeArray` "ObjectTypeQuery3" :!type "EObjectTypeQuery Enum")))
        (if _returnvalue_2
          (`GameplayStatics.ApplyDamage` (`.HitActor` (`GameplayStatics.BreakHitResult` _outhit)) 10.0))))))

(fn `UserConstructionScript`)